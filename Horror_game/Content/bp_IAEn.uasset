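; Enemy AI character Blueprint that spots the player and performs a melee punch.
; Pawn sensing sets the "seeplayer" blackboard key when it sees a pawn tagged Player, and nothing here clears it.
; The attackplayer event, guarded against re-entry until the montage completes, plays a hook punch.
; As the montage starts, it sphere-traces forward from the attack point for WorldStatic objects and damages the hit actor.
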(event `self.PawnSensing.OnSeePawn`
  (params (Pawn :type "Pawn Object Reference"))
  (if (`self.ActorHasTag` Pawn "Player")
    (`BlackboardComponent.SetValueAsBool` (`AIBlueprintHelperLibrary.GetBlackboard` (`AIBlueprintHelperLibrary.GetAIController` self)) "seeplayer" true)))

(event `attackplayer`
  (bind _attackpoint (`self.attackpoint`))
  (bind _returnvalue (`SceneComponent.K2_GetComponentLocation` _attackpoint))
  (if (not (`self.attaking`))
    (set `self.attaking` true)
    (`|PlayMontage` (`self.Mesh`) "/Game/iafolder/Hook_Punch_Montage.Hook_Punch_Montage"
      (:`then`
        (bind (_outhit _returnvalue_2) (`KismetSystemLibrary.SphereTraceSingleForObjects` :`Start` _returnvalue :`End` (+ _returnvalue (* (`KismetMathLibrary.GetForwardVector` (`SceneComponent.K2_GetComponentRotation` _attackpoint)) 70.0)) :`Radius` 25.0 :`ObjectTypes` (`|MakeArray` "ObjectTypeQuery1" :!type "EObjectTypeQuery Enum") :`DrawDebugType` "ForDuration"))
        (if _returnvalue_2
          (`GameplayStatics.ApplyDamage` (`.HitActor` (`GameplayStatics.BreakHitResult` _outhit)) 10.0)))
      (:`OnCompleted`
        (set `self.attaking` false)))))

(fn `UserConstructionScript`)