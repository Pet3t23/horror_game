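; Interactable door Blueprint that teleports the player between the inside and outside of a space.
; Each Interact flips the Inside flag and moves player 0 to the location and rotation of one of two reference points.
; Entering uses REF and exiting uses REFinside.
; Both branches also set the Door's relative rotation to zero.
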(event `/Game/blueprints/bp_interaction.interact`
  (bind (_returnvalue_location _returnvalue_rotation) (`KismetMathLibrary.BreakTransform` (`SceneComponent.K2_GetComponentToWorld` (`self.REF`))))
  (bind (_returnvalue_location_2 _returnvalue_rotation_2) (`KismetMathLibrary.BreakTransform` (`SceneComponent.K2_GetComponentToWorld` (`self.REFinside`))))
  (if (not (`self.inside`))
    (set `self.inside` true)
    (`self.K2_SetActorTransform` (`GameplayStatics.GetPlayerCharacter` 0) (`KismetMathLibrary.MakeTransform` _returnvalue_location _returnvalue_rotation) false false)
    (`SceneComponent.K2_SetRelativeRotation` :`self` (`self.door`))
    (else
      (set `self.inside` false)
      (`self.K2_SetActorTransform` (`GameplayStatics.GetPlayerCharacter` 0) (`KismetMathLibrary.MakeTransform` _returnvalue_location_2 _returnvalue_rotation_2) false false)
      (`SceneComponent.K2_SetRelativeRotation` :`self` (`self.door`)))))

(fn `UserConstructionScript`)